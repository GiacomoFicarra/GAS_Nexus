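; BP_Weapon_Hat is a hat weapon Blueprint that customizes the spawn point location of its parent weapon class.
; Its GetSpawnPointLocation override casts the Instigator to BP_NexusPlayer and returns the world location of that player's HatProjectileSpawn component.
; Any other instigator falls back to the parent implementation.
; The event graph and construction script add no logic of their own.
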(event EventBeginPlay
  (|CallParentFunction) ; This node is disabled and will not be called.\nDrag off pins to build functionality.
)

(event Collision|EventActorBeginOverlap
  (params (OtherActor :type Actor%20Object%20Reference))
  (|CallParentFunction OtherActor) ; This node is disabled and will not be called.\nDrag off pins to build functionality.
)

(event EventTick
  (params (DeltaSeconds :type Float%20%28single-precision%29))
  (|CallParentFunction DeltaSeconds) ; This node is disabled and will not be called.\nDrag off pins to build functionality.
)

(fn ConstructionScript
  (|CallParentFunction))

(fn GetSpawnPointLocation
  (bind _asbp_nexus_player (Utilities|Casting|CastToBP_NexusPlayer (Variables|Default|GetInstigator))
    (:then
      (return (Transformation|GetWorldLocation (Variables|/Game/GameplayAbilitySystem/Character/BP_NexusPlayer.BP_NexusPlayer_C|GetHatProjectileSpawn _asbp_nexus_player))))
    (:CastFailed
      (bind _location (|CallParentFunction))
      (return _location))))