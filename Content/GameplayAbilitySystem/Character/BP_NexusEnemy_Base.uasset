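; Base Blueprint for Gameplay Ability System enemies, with an overhead-bar widget that is removed on death.
; On possession it waits a tick, sends an axe-equip gameplay event, starts a looping timer and applies a shield-fill effect.
; Attack focuses the AI on the first player and looks up melee abilities by tag, but the random ability activation is disconnected, so no attack fires here.
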(event Custom|Attack
  (bind _attacktarget (CallFunction|GetAttackTarget))
  (AI|SetFocus (AI|GetAIController self) _attacktarget)
  (bind _outabilityhandles (GameplayAbilities|FindAllAbilitieswithTags (Variables|Default|GetAbilitySystemComponent) "(GameplayTags=((TagName=\"GameplayAbility.MeleeAttack\")))" true)))

(event EventBeginPlay
  (bind _returnvalue (UserInterface|CreateWidget "/Game/Widgets/Enemy/WBG_EnemyBars.WBG_EnemyBars_C" 0 self))
  (UserInterface|SetWidget (Variables|Default|GetHealthbarWidgetComponent) _returnvalue))

(event EventHandleDeath
  (|CallParentFunction)
  (bind _healthbarwidgetcomponent (Variables|Default|GetHealthbarWidgetComponent)
    (:then
      (Components|DestroyComponent _healthbarwidgetcomponent))
    (:else)))

(event EventPossessed
  (params (NewController :type Controller%20Object%20Reference))
  (Utilities|FlowControl|DelayUntilNextTick)
  (Ability|SendGameplayEventtoActor self "(TagName=\"Event.ActivateAbility.EquipWeapon\")" (Utilities|Struct|MakeGameplayEventData "(GameplayTags=((TagName=\"Weapon.Melee.Axe\")))"))
  (Utilities|Time|SetTimerbyEvent (EventDispatchers|CreateEvent :!event Custom|Attack) 3.0 true)
  (GameplayEffects|ApplyGameplayEffectToSelf :self (Variables|Default|GetAbilitySystemComponent) :GameplayEffectClass "/Game/GameplayAbilitySystem/Effects/GE_FillShield.GE_FillShield_C"))

(fn ConstructionScript)

(fn GetAttackTarget
  (return (Game|GetPlayerCharacter 0)))