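; Base gameplay ability for reactive status effects that trigger when a debuff applied to a target reaches its stack limit.
; On activation it listens for effects applied to targets and checks each for the data asset's debuff tag and max stack count.
; A match applies the data asset's status effect to that target with its configured duration.
; A pass-through ModifyEffectSpecBeforeApplication function lets children adjust the spec first.
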(event Ability|EventActivateAbility
  (bind (_asynctaskproxy _target _spechandle _activehandle) (Ability|Tasks|WaitGameplayEffectAppliedToTarget :OptionalExternalOwner 0)
    (:OnApplied
      (bind _returnvalue (Class|AbilitySystemBlueprintLibrary|IsActiveGameplayEffectHandleValid _activehandle))
      (if _returnvalue
        (Utilities|IsValid (Ability|GameplayEffect|GetGameplayEffectfromActiveEffectHandle _activehandle)
          (:Is%20Valid
            (if (GameplayTags|HasMatchingGameplayTag (Ability|GameplayEffect|GetGameplayEffectfromActiveEffectHandle _activehandle) (Variables|/Game/GameplayAbilitySystem/Data/PDA_StatusEffect.PDA_StatusEffect_C|GetDebuffTag (Variables|Default|GetStatusEffectDA)))
              (bind _returnvalue_2 (Ability|GameplayEffect|GetActiveGameplayEffectStackCount _activehandle))
              (if (>= _returnvalue_2 (Variables|/Game/GameplayAbilitySystem/Data/PDA_StatusEffect.PDA_StatusEffect_C|GetMaxStackCount (Variables|Default|GetStatusEffectDA)))
                (bind _returnvalue_3 (Ability|GameplayEffect|SetDuration (Ability|MakeOutgoingGameplayEffectSpec (Variables|/Game/GameplayAbilitySystem/Data/PDA_StatusEffect.PDA_StatusEffect_C|GetGameplayEffectClass (Variables|Default|GetStatusEffectDA))) (Variables|/Game/GameplayAbilitySystem/Data/PDA_StatusEffect.PDA_StatusEffect_C|GetStatusDuration (Variables|Default|GetStatusEffectDA))))
                (bind _specout (CallFunction|ModifyEffectSpecBeforeApplication _returnvalue_3))
                (GameplayEffects|ApplyGameplayEffectSpecToTarget _specout (Ability|TargetData|AbilityTargetDatafromActor _target))))))))))

(fn ModifyEffectSpecBeforeApplication
  (params (SpecIn :type Gameplay%20Effect%20Spec%20Handle%20Structure))
  (return SpecIn))