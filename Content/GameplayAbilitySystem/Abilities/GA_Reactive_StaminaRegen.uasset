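; Reactive Gameplay Ability that manages delayed stamina regeneration on its avatar by watching for attribute changes.
; Each change compares stamina to the cached value; a drop removes the active GE_Status_StaminaRegen and reapplies it after a short delay.
; Every drop starts its own delay without cancelling earlier ones, and only the latest effect handle is stored.
; Otherwise, stamina reaching a compared attribute value, presumably the maximum, removes the effect.
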(event Ability|EventActivateAbility
  (Variables|Default|SetOldStamina (.ReturnValue (Ability|Attribute|GetFloatAttribute (Ability|GetAvatarActorfromActorInfo) "(AttributeName=\"Stamina\",Attribute=/Script/GAS_Nexus.BasicAttributeSet:Stamina,AttributeOwner=\"/Script/CoreUObject.Class'/Script/GAS_Nexus.BasicAttributeSet'\")")))
  (|WaitforAttributeChange :Attribute "(AttributeName=\"Stamina\",Attribute=/Script/GAS_Nexus.BasicAttributeSet:Stamina,AttributeOwner=\"/Script/CoreUObject.Class'/Script/GAS_Nexus.BasicAttributeSet'\")" :TriggerOnce false :OptionalExternalOwner 0
    (:OnChange
      (bind _output_get (Variables|Default|SetNewStamina (.ReturnValue (Ability|Attribute|GetFloatAttribute (Ability|GetAvatarActorfromActorInfo) "(AttributeName=\"Stamina\",Attribute=/Script/GAS_Nexus.BasicAttributeSet:Stamina,AttributeOwner=\"/Script/CoreUObject.Class'/Script/GAS_Nexus.BasicAttributeSet'\")"))))
      (Utilities|FlowControl|Sequence
        (:then_0
          (if (< _output_get (Variables|Default|GetOldStamina))
            (Ability|RemoveGameplayEffectFromOwnerWithHandle (Variables|Default|GetStaminaRegenEffectHandle))
            (Ability|Tasks|WaitDelay 1.0
              (:OnFinish
                (bind _returnvalue (Ability|ApplyGameplayEffectToOwner "/Game/GameplayAbilitySystem/Effects/GE_Status_StaminaRegen.GE_Status_StaminaRegen_C" (Ability|GetAbilityLevel)))
                (Variables|Default|SetStaminaRegenEffectHandle _returnvalue)))
            (elif (>= (Variables|Default|GetNewStamina) (.ReturnValue (Ability|Attribute|GetFloatAttribute (Ability|GetAvatarActorfromActorInfo) "(AttributeName=\"MaxStamina\",Attribute=/Script/GAS_Nexus.BasicAttributeSet:MaxStamina,AttributeOwner=\"/Script/CoreUObject.Class'/Script/GAS_Nexus.BasicAttributeSet'\")")))
              (Ability|RemoveGameplayEffectFromOwnerWithHandle (Variables|Default|GetStaminaRegenEffectHandle)))))
        (:then_1
          (Variables|Default|SetOldStamina (Variables|Default|GetNewStamina)))))))