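; Gameplay ability for an axe melee combo, extending a parent melee attack with timed input chaining and escalating damage.
; Montage start resets the count and listens for gameplay events that open and close the combo window, while a self-re-arming input wait records whether presses land inside it.
; Window close increments the count or ends the ability; owners without a player controller always continue.
; Hit-scan start scales damage by combo count before running parent logic.
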(event Custom|WaitContinueCombo
  (Ability|Tasks|WaitInputPress false
    (:OnPress
      (Variables|Default|SetReceivedInputAtRightTime (Variables|Default|GetIsWithinComboWindow))
      (CallFunction|WaitContinueCombo))))

(event Ability|EventActivateAbility
  (|CallParentFunction)
  (Variables|Default|SetAlwaysContinueCombo (not (Class|NexusGameplayAbility|HasPC))))

(event Ability|EventOnEndAbility
  (params (bWasCancelled :type Boolean))
  (|CallParentFunction bWasCancelled) ; This node is disabled and will not be called.\nDrag off pins to build functionality.
)

(event EventMontageStarted
  (Variables|Default|SetComboCount 1)
  (Ability|Tasks|WaitGameplayEvent "(TagName=\"Event.ContinueCombo.Start\")" 0
    (:then
      (Ability|Tasks|WaitGameplayEvent "(TagName=\"Event.ContinueCombo.End\")" 0
        (:then
          (CallFunction|WaitContinueCombo))
        (:EventReceived
          (Variables|Default|SetIsWithinComboWindow false)
          (if (or (Variables|Default|GetReceivedInputAtRightTime) (Variables|Default|GetAlwaysContinueCombo))
            (Math|Integer|IncrementInt (Variables|Default|GetComboCount))
            (else
              (Ability|EndAbility))))))
    (:EventReceived
      (Variables|Default|SetIsWithinComboWindow true)
      (Variables|Default|SetReceivedInputAtRightTime false))))

(event EventHandleHitScanStart
  (Variables|Default|SetDamageMagnitude (* (Variables|Default|GetComboMultiplier) (Variables|Default|GetComboCount)))
  (|CallParentFunction))